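; Player Blueprint that lets the character interact with nearby objects in the world.
; Box overlap events maintain CollisionObjects, a list of overlapping actors without duplicates.
; The Interact event takes the first tracked actor, casts it to Interactable and calls OnInteract with itself as an RPGPlayer, then exits the loop.
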(event `self.Interact`
  (for _array_element (`self.CollisionObjects`)
    (bind _asinteractable (cast `Interactable` _array_element))
    (bind _asrpgplayer (cast `RPGPlayer` self))
    (`Interactable.OnInteract` _asinteractable _asrpgplayer)
    (break)))

(event `self.Box.OnComponentBeginOverlap`
  (params (OverlappedComponent :type "PrimitiveComponent Object Reference") (OtherActor :type "Actor Object Reference") (OtherComp :type "PrimitiveComponent Object Reference") (OtherBodyIndex :type Integer) (bFromSweep :type Boolean) (SweepResult :type "HitResult Structure (by ref)"))
  (if (not (`KismetArrayLibrary.Array_Contains` (`self.CollisionObjects`) OtherActor))
    (`KismetArrayLibrary.Array_Add` (`self.CollisionObjects`) OtherActor)))

(event `self.Box.OnComponentEndOverlap`
  (params (OverlappedComponent :type "PrimitiveComponent Object Reference") (OtherActor :type "Actor Object Reference") (OtherComp :type "PrimitiveComponent Object Reference") (OtherBodyIndex :type Integer))
  (`KismetArrayLibrary.Array_RemoveItem` (`self.CollisionObjects`) OtherActor))

(fn `UserConstructionScript`)